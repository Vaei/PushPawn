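; BP_PusheeComponent lets its owning pawn be pushed by other actors, supplying the data a push system queries.
; It allows pushing whenever the pawn and pusher are valid, and reports velocity, ground state and a collision shape from the default root capsule.
; Acceleration comes from a Character owner's movement component, with other pawns returning their velocity in its place.
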(fn K2CanbePushedby
  (params (PusherActor :type Actor%20Object%20Reference))
  (return (and (CallFunction|IsPushable) (Utilities|IsValid PusherActor))))

(fn K2GetPusheeAcceleration
  (bind _characterowner (Variables|Default|GetCharacterOwner)
    (:then
      (return (Pawn|Components|CharacterMovement|GetCurrentAcceleration (Variables|/Script/Engine.Character|GetCharacterMovement _characterowner))))
    (:else
      (bind _pawnowner (Variables|Default|GetPawnOwner)
        (:then
          (return (Transformation|GetVelocity _pawnowner)))
        (:else
          (return "0, 0, 0"))))))

(fn K2GetPusheeCollisionShape
  (bind _pawnowner (Variables|Default|GetPawnOwner)
    (:then
      (if (.ReturnValue (Class|PushStatics|GetDefaultCapsuleRootComponent _pawnowner))
        (return (Utilities|Struct|MakePushPawnCollisionShapeHelper "Capsule" (.CapsuleRadius (Class|PushStatics|GetDefaultCapsuleRootComponent _pawnowner)) (.CapsuleHalfHeight (Class|PushStatics|GetDefaultCapsuleRootComponent _pawnowner))))
        (else
          (return (Utilities|Struct|MakePushPawnCollisionShapeHelper "None")))))
    (:else)))

(fn K2IsPushable
  (return (Utilities|IsValid (Variables|Default|GetPawnOwner))))

(fn K2GetPusheeVelocity
  (bind _pawnowner (Variables|Default|GetPawnOwner)
    (:then
      (return (Transformation|GetVelocity _pawnowner)))
    (:else
      (return "0, 0, 0"))))

(fn K2IsPusheeMovingonGround
  (bind _pawnowner (Variables|Default|GetPawnOwner)
    (:then
      (return (Class|PushStatics|IsPawnMovingonGround _pawnowner)))
    (:else
      (return true))))